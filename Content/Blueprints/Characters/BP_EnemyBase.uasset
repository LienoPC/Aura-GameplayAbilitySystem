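; BP_EnemyBase is the enemy character base Blueprint, handling spawn scale-up, dissolve effects, motion warp facing and loot drops.
; Timelines scale the mesh on BeginPlay and drive the Dissolve parameter on supplied body and weapon dynamic materials.
; UpdateWarpTarget sets the FacingTarget location for Motion Warping.
; SpawnLoot gets tiered loot items, then a looping timer spawns them in an evenly spaced ring, optionally passing enemy level to AuraEffectActor drops.
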(event Custom|SpawnLootItem
  (bind _lootitems (Variables|Default|GetLootItems))
  (bind _itemsspawnlootcount (Variables|Default|GetItemsSpawnLootCount))
  (bind _output (Utilities|Array|Get(acopy) _lootitems _itemsspawnlootcount))
  (if (< (Variables|Default|GetItemsSpawnLootCount) (- (Utilities|Array|Length (Variables|Default|GetLootItems)) 1))
    (bind _returnvalue (Game|SpawnActorfromClass (.lootclass _output) (CallFunction|GetLootTransform (Variables|Default|GetItemsSpawnLootCount)) "AlwaysSpawn" "MultiplyWithRoot" 0 0))
    (Math|Integer|IncrementInt (Variables|Default|GetItemsSpawnLootCount)
      (:%20%20
        (Utilities|IsValid _returnvalue
          (:Is%20Valid
            (if (.blootleveloverride _output)
              (bind _asaura_effect_actor (Utilities|Casting|CastToAuraEffectActor _returnvalue))
              (Variables|/Script/Aura.AuraEffectActor|SetActorLevel _asaura_effect_actor (Math|Conversions|ToFloat(Integer) (Variables|Default|GetLevel))))))))
    (else
      (Utilities|Time|ClearandInvalidateTimerbyHandle (Variables|Default|GetLootTimerHandle)))))

(event EventBeginPlay
  (bind _scaletrack (Timeline|Timeline Play)
    (:Update
      (Transformation|SetRelativeScale3D (Variables|Character|GetMesh) (Math|Vector|MakeVector _scaletrack _scaletrack _scaletrack)))))

(event Collision|EventActorBeginOverlap
  (params (OtherActor :type Actor%20Object%20Reference)))

(event EventTick
  (params (DeltaSeconds :type Float%20%28single-precision%29)))

(event EventStartDissolvingTimeline
  (params (DynamicMaterialInstance :type Material%20Instance%20Dynamic%20Object%20Reference))
  (bind _dissolvetrack (Timeline|Dissolve PlayFromStart)
    (:Update
      (Rendering|Material|SetScalarParameterValue DynamicMaterialInstance "Dissolve" _dissolvetrack :!class /Script/Engine.MaterialInstanceDynamic))))

(event EventStartWeaponDissolvingTimeline
  (params (DynamicMaterialInstance :type Material%20Instance%20Dynamic%20Object%20Reference))
  (bind _weapondissolve (Timeline|WeaponDissolve PlayFromStart)
    (:Update
      (Rendering|Material|SetScalarParameterValue DynamicMaterialInstance "Dissolve" _weapondissolve :!class /Script/Engine.MaterialInstanceDynamic))))

(event EventUpdateWarpTarget
  (params (TargetPosition :type Vector%20%28by%20ref%29 :default "0, 0, 0"))
  (Class|MotionWarpingComponent|AddorUpdateWarpTargetfromLocation (Variables|Default|GetMotionWarping) "FacingTarget" TargetPosition))

(event EventSpawnLoot
  (bind _returnvalue (Class|AuraAbilitySystemLibrary|GetLootTiers self))
  (Utilities|IsValid _returnvalue
    (:Is%20Valid
      (bind _returnvalue_2 (Class|LootTiers|GetLootItems _returnvalue))
      (bind _output_get (Variables|Default|SetLootItems _returnvalue_2))
      (Variables|Default|SetLootRotations (CallFunction|GetLootRotations _output_get))
      (Variables|Default|SetItemsSpawnLootCount 0)
      (bind _returnvalue_3 (Utilities|Time|SetTimerbyEvent (delegate Custom|SpawnLootItem) 0.1 true))
      (Variables|Default|SetLootTimerHandle _returnvalue_3)
      (CallFunction|SpawnLootItem))))

(fn ConstructionScript)

(fn GetLootRotations
  (params (TargetArray :type Array%20of%20Loot%20Item%20Structures))
  (return (Class|AuraAbilitySystemLibrary|EvenlySpacedRotators (Transformation|GetActorForwardVector) (Math|Vector|VectorUp) 3.6e+02 (Utilities|Array|Length TargetArray))))

(fn GetLootTransform
  (params (LoopCount%201 :type Integer))
  (bind _lootrotations (Variables|Default|GetLootRotations))
  (bind _output (Utilities|Array|Get(acopy) _lootrotations LoopCount%201))
  (return (Math|Transform|MakeTransform (+ (* (Math|Vector|GetForwardVector _output) (Variables|Default|GetItemsSpawnDistance)) (Transformation|GetActorLocation)) _output)))