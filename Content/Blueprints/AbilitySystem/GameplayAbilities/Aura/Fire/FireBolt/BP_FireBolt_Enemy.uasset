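; Enemy Fire Bolt actor that explodes and destroys itself when it stops moving.
; Tick compares this frame's location with the last and, below a minimum travel distance, plays the impact sound and Niagara fire explosion before destroying the actor.
; Sphere begin and end overlaps are forwarded to OnOverlap and OnEndOverlap, whose logic is not defined in this graph.
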(event OnComponentBeginOverlap(Sphere)
  (params (OverlappedComponent :type Primitive%20Component%20Object%20Reference) (OtherActor :type Actor%20Object%20Reference) (OtherComp :type Primitive%20Component%20Object%20Reference) (OtherBodyIndex :type Integer) (bFromSweep :type Boolean) (SweepResult :type Hit%20Result%20Structure%20%28by%20ref%29))
  (Class|AuraProjectile|OnOverlap OtherActor))

(event OnComponentEndOverlap(Sphere)
  (params (OverlappedComponent :type Primitive%20Component%20Object%20Reference) (OtherActor :type Actor%20Object%20Reference) (OtherComp :type Primitive%20Component%20Object%20Reference) (OtherBodyIndex :type Integer))
  (Class|AuraProjectile|OnEndOverlap OtherActor))

(event EventBeginPlay)

(event Collision|EventActorBeginOverlap
  (params (OtherActor :type Actor%20Object%20Reference)))

(event EventTick
  (params (DeltaSeconds :type Float%20%28single-precision%29))
  (bind _returnvalue (Transformation|GetActorLocation))
  (Variables|Default|SetLocationLastFrame (Variables|Default|GetLocationThisFrame))
  (Variables|Default|SetLocationThisFrame (Transformation|GetActorLocation))
  (if (< (Math|Vector|VectorLength (- (Variables|Default|GetLocationThisFrame) (Variables|Default|GetLocationLastFrame))) (Variables|Default|GetMinDistancePerFrame))
    (Audio|SpawnSoundatLocation "/Game/Assets/Sounds/Abilities/FireBolt/sfx_FireBolt_Impact.sfx_FireBolt_Impact" _returnvalue "0, 0, 0" 1.0 1.0 0.0 0 0)
    (Niagara|SpawnSystematLocation "/Game/Assets/Effects/Projectiles/FireExplosion/NS_FireExplosion1.NS_FireExplosion1" _returnvalue)
    (Actor|DestroyActor)))

(fn ConstructionScript)