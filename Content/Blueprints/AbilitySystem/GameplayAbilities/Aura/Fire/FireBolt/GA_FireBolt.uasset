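; GA_FireBolt is a gameplay ability that casts homing fire bolts at the target under the mouse.
; On activation it commits, reads the mouse target data and sets the avatar's warp target through the combat interface.
; It plays the cast montage and waits for its gameplay event to spawn projectiles from the ranged socket with overridden pitch, homing on the hit actor.
; The ability ends when the montage completes, is interrupted or is cancelled.
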(event Ability|EventActivateAbility
  (Ability|CommitAbility)
  (bind _datahandle (|TargetDataUnderMouse)
    (:ValidData
      (Variables|Default|SetTargetActor (.HitActor (Collision|BreakHitResult (Ability|TargetData|GetHitResultfromTargetData _datahandle))))
      (bind _ascombat_interface (Utilities|Casting|CastToCombatInterface (Ability|GetAvatarActorfromActorInfo)))
      (Class|CombatInterface|UpdateWarpTarget _ascombat_interface (.Location (Collision|BreakHitResult (Ability|TargetData|GetHitResultfromTargetData _datahandle))))
      (|PlayMontageandWaitProxy "None" "/Game/Assets/Characters/Aura/Animations/Abilities/AM_Cast_FireBolt.AM_Cast_FireBolt" 1.0 "None" false 1.0 0.0 false
        (:then
          (Ability|Tasks|WaitGameplayEvent "(TagName=\"Event.Montage.FireBolt\")" 0
            (:EventReceived
              (Class|AuraFireBolt|SpawnProjectiles (.Location (Collision|BreakHitResult (Ability|TargetData|GetHitResultfromTargetData _datahandle))) (GameplayTags|MakeLiteralGameplayTag "(TagName=\"CombatSocket.Ranged\")") true 45.0 (Variables|Default|GetTargetActor)))))
        (:OnCompleted
          (Ability|EndAbility :!label _label))
        (:OnInterrupted
          (goto _label))
        (:OnCancelled
          (goto _label))))))

(event Ability|EventOnEndAbility
  (params (bWasCancelled :type Boolean)))