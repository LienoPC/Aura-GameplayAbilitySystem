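; Arcane Shards gameplay ability: shows a magic circle, then casts a series of damaging shards at the mouse location on input press.
; A spawned point collection supplies randomly rotated ground points, and the cast montage uses a warp target.
; The montage event hides the circle and starts a looping timer, placing one shard per point.
; Each shard damages nearby living entities except the caster, with outward knockback, and fires a GameplayCue until cleanup.
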(event Custom|SpawnShard
  (bind _returnvalue (Ability|GetAvatarActorfromActorInfo))
  ;[0.15 0.15 0.15 0.5] Spawn shard at point
  (if (< (Variables|Default|GetCountPointIteration) (Variables|Default|GetMaxNumShards))
    (CallFunction|StoreShardSpawnLocation)
    (bind _outentities (Class|AuraAbilitySystemLibrary|GetLiveEntitiesWithinRadius _returnvalue (Variables|Default|GetShardSpawnLocation) (Variables|Default|GetRadialDamageOuterRadius) (Utilities|Array|MakeArray _returnvalue)))
    (bind _output_get (Variables|Default|SetOverlappingEnemies _outentities))
    (for _array_element _output_get
      (Class|AuraAbilitySystemLibrary|ApplyDamageEffect (Class|DamageGameplayAbility|MakeDamageEffectParamsfromClassDefaults _array_element (Variables|Default|GetShardSpawnLocation) true (- (Transformation|GetActorLocation _array_element) (Variables|Default|GetShardSpawnLocation)) false (- (Transformation|GetActorLocation _array_element) (Variables|Default|GetShardSpawnLocation)) true 35.0)))
    (Math|Integer|IncrementInt (Variables|Default|GetCountPointIteration)
      (:%20%20
        (Class|GameplayAbility|ExecuteGameplayCuewithParams "(TagName=\"GameplayCue.ArcaneShards\")" (Ability|GameplayCue|MakeGameplayCueParameters :Location (Variables|Default|GetShardSpawnLocation)))))
    (else
      ;[0.15 0.15 0.15 0.5] End and clean ability
      (Utilities|Time|ClearandInvalidateTimerbyHandle (Variables|Default|GetShardSpawnTimer))
      (Utilities|FlowControl|Delay 0.5)
      (Variables|Default|SetCountPointIteration 0)
      (Actor|DestroyActor (Variables|Default|GetPointCollection))
      (Ability|EndAbility))))

(event Ability|EventActivateAbility
  (Utilities|FlowControl|Sequence
    (:then_0
      (Class|PlayerInterface|ShowMagicCircle(Message) (Ability|GetAvatarActorfromActorInfo) 0))
    (:then_1
      (Ability|Tasks|WaitInputPress false
        (:OnPress
          (bind _datahandle (|TargetDataUnderMouse)
            (:ValidData
              (bind _output_get (Variables|Default|SetMouseHitLocation (.impactpoint (Ability|TargetData|GetHitResultfromTargetData _datahandle))))
              (bind _returnvalue (Game|SpawnActorfromClass "/Game/Blueprints/AbilitySystem/GameplayAbilities/Aura/Arcane/ArcaneShards/BP_ArcaneShardsPointCollection.BP_ArcaneShardsPointCollection_C" (Math|Transform|MakeTransform _output_get "0, 0, 0" "1.000000,1.000000,1.000000") "Undefined" "MultiplyWithRoot" 0 0))
              (Variables|Default|SetGroundPoints (Class|PointCollection|GetGroundPoints _returnvalue (Variables|Default|GetMouseHitLocation) 0 (Math|Random|RandomFloatinRange 0.0 5e+02)))
              (Variables|Default|SetPointCollection _returnvalue)
              (Class|CombatInterface|UpdateWarpTarget(Message) (Ability|GetAvatarActorfromActorInfo) (Variables|Default|GetMouseHitLocation))
              ;[0.15 0.15 0.15 0.5] PlayMontage and Wait for Event
              (|PlayMontageandWaitProxy "None" "/Game/Assets/Characters/Aura/Animations/Abilities/AM_Cast_ArcaneShards.AM_Cast_ArcaneShards" 1.0 "None" false 1.0 0.0 false
                (:then
                  (Ability|Tasks|WaitGameplayEvent "(TagName=\"Event.Montage.ArcaneShards\")" 0 true
                    (:EventReceived
                      (bind _returnvalue_2 (Utilities|Time|SetTimerbyEvent (delegate Custom|SpawnShard) (Variables|Default|GetShardSpawnDeltaTime) true))
                      (Variables|Default|SetShardSpawnTimer _returnvalue_2)
                      (CallFunction|SpawnShard)
                      (Class|PlayerInterface|HideMagicCircle(Message) (Ability|GetAvatarActorfromActorInfo)))))))))))))

(event Ability|EventOnEndAbility
  (params (bWasCancelled :type Boolean)))

(fn StoreShardSpawnLocation
  (Variables|Default|SetShardSpawnLocation (Transformation|GetWorldLocation (Utilities|Array|Get(acopy) (Variables|Default|GetGroundPoints) (Variables|Default|GetCountPointIteration))))
  (return))