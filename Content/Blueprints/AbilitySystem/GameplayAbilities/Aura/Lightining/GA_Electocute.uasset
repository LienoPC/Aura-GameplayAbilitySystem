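; Electrocute gameplay ability: a held lightning beam that strikes the target under the mouse and chains to nearby targets.
; A montage event locks movement, adds ShockLoop cues to the targets and starts a looping timer that commits cost and applies set-by-caller lightning damage.
; Releasing input, after a minimum hold time, clears cues, restores movement and commits cooldown.
; Target deaths trigger cleanup, dropping secondary targets individually or shutting down the beam for the primary.
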(event Custom|DamageAndCost
  (bind _returnvalue (Ability|CommitAbilityCost false))
  (if _returnvalue
    (CallFunction|ApplyDamagetoAllTargets)))

(event Ability|EventActivateAbility
  (if (Utilities|DoesObjectImplementInterface (Ability|GetAvatarActorfromActorInfo) "/Script/Aura.CombatInterface")
    ;[0.09771 0.5825 1] Store Mouse Data Variables
    (bind _datahandle (|TargetDataUnderMouse)
      (:ValidData
        (Class|AuraBeamSpell|StoreMouseDataInfo (Ability|TargetData|GetHitResultfromTargetData _datahandle))
        (Class|AuraBeamSpell|StoreOwnerVariables)
        (Utilities|FlowControl|Sequence
          (:then_0
            (Variables|/Script/Engine.PlayerController|SetbShowMouseCursor (Variables|Default|GetOwnerPlayerController) false)
            (Class|CombatInterface|UpdateWarpTarget(Message) (Ability|GetAvatarActorfromActorInfo) (Variables|Default|GetMouseHitLocation))
            (GameplayCue|ExecuteGameplayCue :GameplayCueTag "(TagName=\"GameplayCue.ShockBurst\")")
            (|PlayMontageandWaitProxy "None" (Variables|Default|GetElectrocuteMontage) 1.0 "None" true 1.0 0.0 false
              (:then
                (Ability|Tasks|WaitGameplayEvent "(TagName=\"Event.Montage.Electrocute\")" 0 true
                  (:EventReceived
                    (CallFunction|InShockLoop)
                    (CallFunction|SpawnElectricBeam)
                    (bind _returnvalue (Utilities|Time|SetTimerbyEvent (delegate Custom|DamageAndCost) (Variables|Default|GetDamageDeltaTime) true))
                    (Variables|Default|SetDamageAndCostTimer _returnvalue))))))
          (:then_1
            (bind _timeheld (Ability|Tasks|WaitInputRelease false)
              (:then
                (Variables|Default|SetTime%20Held _timeheld))
              (:OnRelease
                (if (< (Variables|Default|GetTime%20Held) (Variables|Default|GetMinSpellTime))
                  (Utilities|FlowControl|Delay (- (Variables|Default|GetMinSpellTime) (Variables|Default|GetTime%20Held))))
                (CallFunction|PreparetoEndAbility)
                (Ability|EndAbility)))))))
    (else
      (Ability|EndAbility))))

(event Ability|EventOnEndAbility
  (params (bWasCancelled :type Boolean)))

(event EventOnPrimaryTargetActorDied
  (params (DeadActor :type Actor%20Object%20Reference))
  (Ability|CommitAbilityCooldown false)
  (CallFunction|PreparetoEndAbility))

(event EventOnAdditionalTargetActorDied
  (params (DeadActor :type Actor%20Object%20Reference))
  (bind _additionalactorstocue (Variables|Default|GetAdditionalActorsToCue))
  (bind (_value _returnvalue) (Utilities|Map|Find _additionalactorstocue DeadActor))
  (if _returnvalue
    (GameplayCue|RemoveGameplayCueOnActor(Looping) DeadActor "(TagName=\"GameplayCue.ShockLoop\")" _value)
    (Utilities|Array|RemoveItem (Variables|Default|GetNearby%20Targets) DeadActor)))

(fn PreparetoEndAbility
  (Utilities|Time|ClearandInvalidateTimerbyHandle (Variables|Default|GetDamageAndCostTimer))
  (Variables|/Script/Engine.PlayerController|SetbShowMouseCursor (Variables|Default|GetOwnerPlayerController) true)
  (Class|CombatInterface|SetinShockLoop(Message) (Ability|GetAvatarActorfromActorInfo) false)
  (Pawn|Components|CharacterMovement|SetMovementMode (Variables|/Script/Engine.Character|GetCharacterMovement (Variables|Default|GetOwnerCharacter)) "MOVE_Walking" 0)
  (if (Variables|Default|GetFirst%20Target%20Implements%20Combat%20Interface)
    (GameplayCue|RemoveGameplayCueOnActor(Looping) (Variables|Default|GetMouseHitActor) "(TagName=\"GameplayCue.ShockLoop\")" (Variables|Default|GetFirstTargetCueParams))
    (CallFunction|RemoveCuefromAdditionalActors)
    (Variables|Default|SetTime%20Held 0.0)
    (else
      (GameplayCue|RemoveGameplayCue "(TagName=\"GameplayCue.ShockLoop\")")))
  (Ability|CommitAbilityCooldown false))

(fn InShockLoop
  (Class|CombatInterface|SetinShockLoop(Message) (Ability|GetAvatarActorfromActorInfo) true)
  (Pawn|Components|CharacterMovement|DisableMovement (Variables|/Script/Engine.Character|GetCharacterMovement (Variables|Default|GetOwnerCharacter))))

(fn SpawnElectricBeam
  (bind _mousehitactor (Variables|Default|GetMouseHitActor))
  (bind _returnvalue (Utilities|DoesObjectImplementInterface _mousehitactor "/Script/Aura.CombatInterface"))
  (Class|AuraBeamSpell|TraceFirstTarget (Variables|Default|GetMouseHitLocation))
  (bind _returnvalue_2 (Class|CombatInterface|GetWeapon(Message) (Variables|Default|GetOwnerCharacter)))
  (Variables|Default|SetFirstTargetCueParams (Ability|GameplayCue|MakeGameplayCueParameters :Location (Variables|Default|GetMouseHitLocation) :SourceObject (Variables|Default|GetMouseHitActor) :TargetAttachComponent _returnvalue_2))
  ;[0.15 0.15 0.15 0.5] Is MouseHitActor an Enemy
  (Variables|Default|SetFirst%20Target%20Implements%20Combat%20Interface _returnvalue)
  (if _returnvalue
    (LocalVariables|SetCueTarget (Variables|Default|GetMouseHitActor))
    (else
      (LocalVariables|SetCueTarget (Ability|GetAvatarActorfromActorInfo))))
  (GameplayCue|AddGameplayCueOnActor(Looping) (LocalVariables|GetCueTarget) "(TagName=\"GameplayCue.ShockLoop\")" (Variables|Default|GetFirstTargetCueParams))
  (if (Variables|Default|GetFirst%20Target%20Implements%20Combat%20Interface)
    (bind _nearbytargets (Class|AuraBeamSpell|StoreAdditionalTargets))
    (bind _output_get (Variables|Default|SetNearby%20Targets _nearbytargets))
    (for _array_element _output_get
      (CallFunction|AddShockLoopCuetoAdditionalTarget _array_element))))

(fn AddShockLoopCuetoAdditionalTarget
  (params (Target :type Actor%20Object%20Reference))
  (bind _output_get (LocalVariables|SetTargetActor Target))
  (Utilities|Map|Add (Variables|Default|GetAdditionalActorsToCue) _output_get (Ability|GameplayCue|MakeGameplayCueParameters :Location (Transformation|GetActorLocation _output_get) :SourceObject _output_get :TargetAttachComponent (Variables|/Script/Engine.Actor|GetRootComponent (Variables|Default|GetMouseHitActor))))
  (GameplayCue|AddGameplayCueOnActor(Looping) (LocalVariables|GetTargetActor) "(TagName=\"GameplayCue.ShockLoop\")" (Ability|GameplayCue|MakeGameplayCueParameters :Location (Transformation|GetActorLocation _output_get) :SourceObject _output_get :TargetAttachComponent (Variables|/Script/Engine.Actor|GetRootComponent (Variables|Default|GetMouseHitActor)))))

(fn RemoveCuefromAdditionalActors
  (bind (_keypin _valuepin) (Utilities|Map|ForEachLoop(Map) (Variables|Default|GetAdditionalActorsToCue))
    (:then
      (GameplayCue|RemoveGameplayCueOnActor(Looping) _keypin "(TagName=\"GameplayCue.ShockLoop\")" _valuepin))))

(fn ApplyDamagetoAllTargets
  (bind _mousehitactor (Variables|Default|GetMouseHitActor)
    (:then
      (CallFunction|ApplyDamageSingleTarget _mousehitactor)
      (for _array_element (Variables|Default|GetNearby%20Targets)
        (CallFunction|ApplyDamageSingleTarget _array_element)))
    (:else)))

(fn ApplyDamageSingleTarget
  (params (Target :type Actor%20Object%20Reference))
  (bind _returnvalue (Ability|GetAbilitySystemComponentfromActorInfo))
  (bind _returnvalue_2 (Class|AuraAbilitySystemLibrary|GetAbilitySystemComponent Target))
  (Utilities|IsValid Target
    (:Is%20Valid
      (Utilities|IsValid _returnvalue_2
        (:Is%20Valid
          (bind _returnvalue_3 (Ability|GameplayEffect|AssignTagSetbyCallerMagnitude (GameplayEffects|MakeOutgoingSpec _returnvalue (Variables|Default|GetDamageEffectClass) (Math|Conversions|ToFloat(Integer) (Ability|GetAbilityLevel)) (GameplayEffects|MakeEffectContext _returnvalue)) "(TagName=\"Damage.Lightning\")" (Class|DamageGameplayAbility|GetDamageatLevel)))
          (GameplayEffects|ApplyGameplayEffectSpecToSelf _returnvalue_2 _returnvalue_3))))))