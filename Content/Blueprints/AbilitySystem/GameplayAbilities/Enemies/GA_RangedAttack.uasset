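; Gameplay ability for an enemy ranged attack that fires a projectile at the avatar's combat target.
; On activation it points the warp target at the combat target through CombatInterface, then plays the avatar's attack montages tagged CombatSocket.Ranged.
; A one-shot gameplay event matching the montage tag triggers SpawnProjectile toward the target's location at that moment.
; The ability ends when the montage completes, is interrupted or is cancelled.
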(event Ability|EventActivateAbility
  (bind _returnvalue (Ability|GetAvatarActorfromActorInfo))
  (bind _returnvalue_2 (Ability|GetAvatarActorfromActorInfo))
  (bind _returnvalue_3 (Class|EnemyInterface|GetCombatTarget(Message) _returnvalue_2))
  (bind _ascombat_interface (Utilities|Casting|CastToCombatInterface _returnvalue_2))
  (Class|CombatInterface|UpdateWarpTarget _ascombat_interface (Transformation|GetActorLocation _returnvalue_3))
  (bind _returnvalue_4 (Class|CombatInterface|GetAttackMontages(Message) _returnvalue_2))
  (for _array_element _returnvalue_4
    (if (== (.SocketTag (Utilities|Struct|BreakTaggedMontage _array_element)) "(TagName=\"CombatSocket.Ranged\")")
      (bind _output_get (Variables|Default|SetLocalMontage _array_element))
      (|PlayMontageandWaitProxy "None" (.montage _output_get) 1.0 "None" true 1.0 0.0 false
        (:then
          (Ability|Tasks|WaitGameplayEvent (.montagetag _output_get) 0 true
            (:EventReceived
              (Class|CombatInterface|GetCombatSocketLocation(Message) _returnvalue (.sockettag _output_get))
              (bind _returnvalue_5 (Class|EnemyInterface|GetCombatTarget(Message) _returnvalue))
              (Class|AuraProjectileSpell|SpawnProjectile (Transformation|GetActorLocation _returnvalue_5)))))
        (:OnCompleted
          (Ability|EndAbility :!label _label))
        (:OnInterrupted
          (goto _label))
        (:OnCancelled
          (goto _label))))))

(event Ability|EventOnEndAbility
  (params (bWasCancelled :type Boolean)))