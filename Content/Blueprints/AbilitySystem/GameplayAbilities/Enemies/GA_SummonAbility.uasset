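; Enemy gameplay ability that plays the shaman summon montage and spawns random minion classes at shuffled spawn locations.
; On the montage's gameplay event, it plays a Niagara ground effect at every location, then spawns AI-controlled minions in a staggered, delay-driven loop, facing away from the summoner.
; Each spawn increments the avatar's minion count, and a destroyed-event binding decrements it.
; The ability ends shortly after the last spawn.
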(event Custom|Minion
  (params (DestroyedActor :type Actor%20Object%20Reference))
  (Class|CombatInterface|IncrementMinionCount(Message) (Ability|GetAvatarActorfromActorInfo) -1))

(event Ability|EventActivateAbility
  (bind _spawnlocationindex (Variables|Default|GetSpawnLocationIndex))
  (bind _returnvalue (Class|SummonAbility|GetSpawnLocations))
  (Variables|Default|SetSpawnLocations _returnvalue)
  (Utilities|Array|Shuffle (Variables|Default|GetSpawnLocations))
  (|PlayMontageandWaitProxy "None" "/Game/Assets/Enemies/Shaman/Animations/AM_Shaman_Summon.AM_Shaman_Summon" 1.0 "None" true 1.0 0.0 false
    (:then
      (Ability|Tasks|WaitGameplayEvent "(TagName=\"Montage.Attack.1\")" 0
        (:EventReceived
          (for _array_element (Variables|Default|GetSpawnLocations)
            (Niagara|SpawnSystematLocation "/Game/Assets/Effects/Combat/NS_GroundSummon.NS_GroundSummon" _array_element))
          (Utilities|FlowControl|Delay 0.5)
          (if (< _spawnlocationindex (Utilities|Array|Length (Variables|Default|GetSpawnLocations))) :!label _label
            (Utilities|FlowControl|Delay 0.2)
            (bind _returnvalue_2 (Game|SpawnActorfromClass (.OutItem (Utilities|Array|Random (Variables|Default|GetMinionClasses))) (Math|Transform|MakeTransform (Math|Vector|MakeVector (.X (Math|Vector|BreakVector (Utilities|Array|Get(acopy) (Variables|Default|GetSpawnLocations) _spawnlocationindex))) (.Y (Math|Vector|BreakVector (Utilities|Array|Get(acopy) (Variables|Default|GetSpawnLocations) _spawnlocationindex))) (+ (.Z (Math|Vector|BreakVector (Utilities|Array|Get(acopy) (Variables|Default|GetSpawnLocations) _spawnlocationindex))) 5e+01)) (Math|Rotator|FindLookatRotation (Transformation|GetActorLocation (Ability|GetAvatarActorfromActorInfo)) (Utilities|Array|Get(acopy) (Variables|Default|GetSpawnLocations) _spawnlocationindex)) "1.000000,1.000000,1.000000") "AlwaysSpawn" "MultiplyWithRoot" 0 0))
            (Game|BindEventtoOnDestroyed _returnvalue_2 (delegate Custom|Minion))
            (Pawn|SpawnDefaultController _returnvalue_2)
            (Class|CombatInterface|IncrementMinionCount(Message) (Ability|GetAvatarActorfromActorInfo) 1)
            (Math|Integer|IncrementInt _spawnlocationindex
              (:%20%20
                (goto _label)))
            (else
              (Utilities|FlowControl|Delay 3.0)
              (Ability|EndAbility))))))))

(event Ability|EventOnEndAbility
  (params (bWasCancelled :type Boolean)))