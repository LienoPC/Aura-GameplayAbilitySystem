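; Enemy melee attack ability that turns toward the combat target via a motion-warp update and plays a randomly picked attack montage.
; On the montage's tagged gameplay event, it gathers live entities in a small radius around the attack's combat socket and damages non-friends.
; A single melee impact gameplay cue fires if anything was hit.
; The ability ends after the hit check or when the montage completes or aborts.
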(event Ability|EventActivateAbility
  (bind _returnvalue (Ability|GetAvatarActorfromActorInfo))
  (bind _returnvalue_2 (Ability|GetAvatarActorfromActorInfo))
  (Variables|Default|SetHasHitTarget false)
  (bind _returnvalue_3 (Class|EnemyInterface|GetCombatTarget(Message) _returnvalue))
  (bind _ascombat_interface (Utilities|Casting|CastToCombatInterface _returnvalue))
  (Class|CombatInterface|UpdateWarpTarget _ascombat_interface (Transformation|GetActorLocation _returnvalue_3))
  (bind _returnvalue_4 (Class|CombatInterface|GetAttackMontages(Message) _returnvalue))
  (if (>= (Math|Random|RandomIntegerinRange 0 (- (Utilities|Array|Length _returnvalue_4) 1)) 0)
    (bind _output_get (Variables|Default|SetLocalMontage (Utilities|Array|Get(acopy) _returnvalue_4 (Math|Random|RandomIntegerinRange 0 (- (Utilities|Array|Length _returnvalue_4) 1)))))
    (|PlayMontageandWaitProxy "None" (.montage _output_get) 1.0 "None" true 1.0 0.0 false
      (:then
        (Ability|Tasks|WaitGameplayEvent (.montagetag _output_get) 0
          (:EventReceived
            (bind _returnvalue_5 (Class|CombatInterface|GetCombatSocketLocation(Message) _returnvalue (.sockettag _output_get)))
            (bind _outentities (Class|AuraAbilitySystemLibrary|GetLiveEntitiesWithinRadius _returnvalue _returnvalue_5 6e+01 (Utilities|Array|MakeArray _returnvalue)))
            (for _array_element _outentities
              (if (Class|AuraAbilitySystemLibrary|IsNotFriend (Ability|GetAvatarActorfromActorInfo) _array_element)
                (Class|AuraAbilitySystemLibrary|ApplyDamageEffect (Class|DamageGameplayAbility|MakeDamageEffectParamsfromClassDefaults _array_element "0, 0, 0" false "0, 0, 0" false "0, 0, 0" false 0.0))
                (Variables|Default|SetHasHitTarget true)))
            (if (Variables|Default|GetHasHitTarget)
              (bind _returnvalue_6 (Class|EnemyInterface|GetCombatTarget(Message) _returnvalue_2))
              (Class|GameplayAbility|ExecuteGameplayCuewithParams "(TagName=\"GameplayCue.MeleeImpact\")" (Ability|GameplayCue|MakeGameplayCueParameters :AggregatedSourceTags (GameplayTags|MakeGameplayTagContainerfromTag (.montagetag (Variables|Default|GetLocalMontage))) :Location _returnvalue_5 :EffectCauser _returnvalue_2 :SourceObject _returnvalue_6)))
            (Ability|EndAbility))))
      (:OnCompleted
        (Ability|EndAbility :!label _label))
      (:OnInterrupted
        (goto _label))
      (:OnCancelled
        (goto _label)))
    (else
      (Ability|EndAbility))))

(event Ability|EventOnEndAbility
  (params (bWasCancelled :type Boolean)))