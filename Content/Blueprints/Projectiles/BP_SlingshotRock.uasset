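; BP_SlingshotRock is a slingshot rock projectile that tumbles visually while it exists.
; BeginPlay picks random yaw, roll and pitch speeds, and Tick applies yaw and roll to the static mesh as delta-time-scaled local rotation.
; The pitch speed is multiplied by zero, so it has no effect.
; Collision begin and end overlaps forward the other actor to OnOverlap and OnEndOverlap, which are defined outside these graphs.
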(event OnComponentBeginOverlap(Collision)
  (params (OverlappedComponent :type Primitive%20Component%20Object%20Reference) (OtherActor :type Actor%20Object%20Reference) (OtherComp :type Primitive%20Component%20Object%20Reference) (OtherBodyIndex :type Integer) (bFromSweep :type Boolean) (SweepResult :type Hit%20Result%20Structure%20%28by%20ref%29))
  (Class|AuraProjectile|OnOverlap OtherActor))

(event OnComponentEndOverlap(Collision)
  (params (OverlappedComponent :type Primitive%20Component%20Object%20Reference) (OtherActor :type Actor%20Object%20Reference) (OtherComp :type Primitive%20Component%20Object%20Reference) (OtherBodyIndex :type Integer))
  (Class|AuraProjectile|OnEndOverlap OtherActor))

(event EventBeginPlay
  (bind _returnvalue (Math|Random|RandomFloatinRange -5e+02 5e+02))
  (Variables|Default|SetRandomYawSpeed _returnvalue)
  (Variables|Default|SetRandomRollSpeed _returnvalue)
  (Variables|Default|SetRandomPitchSpeed _returnvalue))

(event Collision|EventActorBeginOverlap
  (params (OtherActor :type Actor%20Object%20Reference)))

(event EventTick
  (params (DeltaSeconds :type Float%20%28single-precision%29))
  (Transformation|AddLocalRotation (Variables|Default|GetStaticMesh) (Math|Rotator|MakeRotator (* DeltaSeconds (Variables|Default|GetRandomRollSpeed)) (* (Variables|Default|GetRandomPitchSpeed) 0.0) (* DeltaSeconds (Variables|Default|GetRandomYawSpeed))) false false))

(fn ConstructionScript)