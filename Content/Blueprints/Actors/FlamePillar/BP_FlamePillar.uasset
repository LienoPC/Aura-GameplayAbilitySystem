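; Flame pillar actor that gives its FireLight a flickering fire glow.
; On BeginPlay it randomly picks one of two timelines, each driving a flame intensity curve into ScaleFrameIntensity, which sets the light to BaseIntensity times that value.
; When either timeline finishes, it picks again at random, so the flicker runs continuously with varying patterns.
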(event Custom|StartTimeline1
  (bind _flameintensity (Timeline|FireTimeline PlayFromStart)
    (:Update
      (CallFunction|ScaleFrameIntensity _flameintensity))
    (:Finished
      (CallFunction|ChooseTimeline))))

(event Custom|StartTimeline2
  (bind _fireint (Timeline|FlameIntensity PlayFromStart)
    (:Update
      (CallFunction|ScaleFrameIntensity _fireint))
    (:Finished
      (CallFunction|ChooseTimeline))))

(event Custom|ChooseTimeline
  (switch int (Math|Random|RandomIntegerinRange 0 1)
    (:Default
      (CallFunction|StartTimeline2))
    (:0
      (CallFunction|StartTimeline1))
    (:1
      (CallFunction|StartTimeline2))))

(event EventBeginPlay
  (CallFunction|ChooseTimeline))

(event Collision|EventActorBeginOverlap
  (params (OtherActor :type Actor%20Object%20Reference)))

(fn ConstructionScript)

(fn ScaleFrameIntensity
  (params (B :type Float%20%28double-precision%29))
  (Rendering|Components|Light|SetIntensity (Variables|Default|GetFireLight) (* (Variables|Default|GetBaseIntensity) B)))